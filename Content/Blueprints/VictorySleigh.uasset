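; VictorySleigh is the win trigger that ends the game when the player reaches it with enough score.
; On actor overlap it casts the other actor to TopDownCharacter and compares the TopDownGameMode's Score against its MaxScore.
; If the score meets or exceeds the maximum, it destroys the character and opens WinLevel.
; A second copy of the destroy-and-load chain, without the score check, is unconnected and never runs.
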(event `self.ReceiveActorBeginOverlap`
  (params (OtherActor :type "Actor Object Reference"))
  (bind _astop_down_character (cast `/Game/TopDownBP/Blueprints/TopDownCharacter` OtherActor))
  (bind _astop_down_game_mode (cast `/Game/TopDownBP/Blueprints/TopDownGameMode` (`GameplayStatics.GetGameMode`)))
  (if (>= (`/Game/TopDownBP/Blueprints/TopDownGameMode.Score` _astop_down_game_mode) (`/Game/TopDownBP/Blueprints/TopDownGameMode.MaxScore` _astop_down_game_mode))
    (`self.K2_DestroyActor` _astop_down_character)
    (`GameplayStatics.OpenLevel` "WinLevel")))

(fn `UserConstructionScript`)